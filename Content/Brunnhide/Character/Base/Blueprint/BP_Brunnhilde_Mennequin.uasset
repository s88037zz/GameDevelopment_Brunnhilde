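; Player character Blueprint for Brunnhilde, handling camera look, jumping, rolling, interaction and the equipment board toggle through the game mode.
; BeginPlay loops synchronously until the game mode's equipment dataset is non-empty, deep-copying each item into the inventory component.
; Jump becomes a roll montage while moving, and rolls wait for any active montage to end.
; A sphere overlap gathers BPI_Interaction actors or components, and Interaction triggers the first.
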(event `self.ReceiveBeginPlay`
  (`self.InitializeFlow`))

(event `RefreshStats`
  ;[1 1 1] ReshStats
)

(event `InputAction|OpenEquipmentBoard`
  (params (Key :type "Key Structure"))
  ;[1 1 1] OpenEquipmentBoard
  (:`Pressed`
    (bind _asbp_brunnhilde_player_game_mode (cast `/Game/Brunnhide/GameMode/BP_Brunnhilde_PlayerGameMode` (`GameplayStatics.GetGameMode`)))
    (`/Game/Brunnhide/GameMode/BPI_UIControl.HandleControlEquipmentBoard` _asbp_brunnhilde_player_game_mode)))

(event `InputAction|TestActions`
  (params (Key :type "Key Structure"))
  ;[1 1 1] TestAction
)

(event `InputAction|Jump`
  (params (Key :type "Key Structure"))
  ;[1 1 1] Jump & dodge
  (:`Pressed`
    (if (`self.HasMovementInput`)
      (`self.PlayRollAnimation`)
      (else
        (`self.Jump`)))))

(event `InputAction|PickUp`
  (params (Key :type "Key Structure"))
  ;[1 1 1] Pickup
)

(event `InputAction|LockEnemy`
  (params (Key :type "Key Structure"))
  ;[1 1 1] LockEnemy
)

(event `InputAction|Roll`
  (params (Key :type "Key Structure"))
  ;[1 1 1] Roll
  (:`Pressed`
    (`self.PlayRollAnimation`)))

(event `self.ReceiveTick`
  (params (DeltaSeconds :type "Float (single-precision)")))

(event `InputAction|Sprint`
  (params (Key :type "Key Structure"))
  ;[1 1 1] Sprint
)

(event `InputAction|Block`
  (params (Key :type "Key Structure"))
  ;[1 1 1] BlockAttack
)

(event `InputAction|ChangeToWeapon01`
  (params (Key :type "Key Structure"))
  ;[1 1 1] Change Weapon
)

(event `InputAxis|TurnAtRate`
  (params (AxisValue :type "Float (single-precision)"))
  ;[1 1 1] MouseInput
  (`self.AddControllerYawInput` AxisValue))

(event `InputAction|ChangeToWeapon02`
  (params (Key :type "Key Structure"))
  ;[1 1 1] Change Weapon
)

(event `InputAxis|LookUpAtRate`
  (params (AxisValue :type "Float (single-precision)"))
  ;[1 1 1] MouseInput
  (`self.AddControllerPitchInput` AxisValue))

(event `InputAction|ChangeToWeapon03`
  (params (Key :type "Key Structure"))
  ;[1 1 1] Change Weapon
)

(event `InputAction|Interaction`
  (params (Key :type "Key Structure"))
  ;[1 1 1] Interaction
  (:`Pressed`
    (if (> (`KismetArrayLibrary.Array_Length` (`self.As BPI Interaction`)) 0)
      (`/Game/Brunnhide/Character/Base/Interface/BPI_Interaction.OnInteraction` (`|GetArrayItem` (`self.As BPI Interaction`)) self)
      (`KismetSystemLibrary.PrintString` "Interaction"))))

(event `self.InteractionSphere.OnComponentBeginOverlap`
  (params (OverlappedComponent :type "PrimitiveComponent Object Reference") (OtherActor :type "Actor Object Reference") (OtherComp :type "PrimitiveComponent Object Reference") (OtherBodyIndex :type Integer) (bFromSweep :type Boolean) (SweepResult :type "HitResult Structure (by ref)"))
  ;[1 1 1] Interaction
  (bind _asbpi_interaction (cast `/Game/Brunnhide/Character/Base/Interface/BPI_Interaction` OtherActor)
    (:`then`
      (`KismetArrayLibrary.Array_AddUnique` (`self.As BPI Interaction`) _asbpi_interaction))
    (:`CastFailed`
      (for _array_element (`self.GetComponentsByInterface` OtherActor "/Game/Brunnhide/Character/Base/Interface/BPI_Interaction.BPI_Interaction_C")
        (`KismetArrayLibrary.Array_AddUnique` (`self.As BPI Interaction`) (cast `/Game/Brunnhide/Character/Base/Interface/BPI_Interaction` _array_element :!pure true))))))

(event `self.InteractionSphere.OnComponentEndOverlap`
  (params (OverlappedComponent :type "PrimitiveComponent Object Reference") (OtherActor :type "Actor Object Reference") (OtherComp :type "PrimitiveComponent Object Reference") (OtherBodyIndex :type Integer))
  ;[1 1 1] Interaction
  (bind _asbpi_interaction (cast `/Game/Brunnhide/Character/Base/Interface/BPI_Interaction` OtherActor)
    (:`then`
      (`KismetArrayLibrary.Array_RemoveItem` (`self.As BPI Interaction`) _asbpi_interaction))
    (:`CastFailed`
      (for _array_element (`self.GetComponentsByInterface` OtherActor "/Game/Brunnhide/Character/Base/Interface/BPI_Interaction.BPI_Interaction_C")
        (`KismetArrayLibrary.Array_RemoveItem` (`self.As BPI Interaction`) (cast `/Game/Brunnhide/Character/Base/Interface/BPI_Interaction` _array_element :!pure true))))))

(fn `GetDesiredRotation`
  (returns (Rotation :type "Rotator Structure"))
  (bind (_returnvalue_x _returnvalue_y _returnvalue_z) (`KismetMathLibrary.BreakVector` (`self.GetLastMovementInputVector`)))
  (`KismetSystemLibrary.PrintString` (`KismetTextLibrary.Conv_TextToString` (`|FormatText` "X:{ x}, Y:{y}, Z:{z}" (`KismetStringLibrary.Conv_DoubleToString` _returnvalue_x) (`KismetStringLibrary.Conv_DoubleToString` _returnvalue_y) (`KismetStringLibrary.Conv_DoubleToString` _returnvalue_z))))
  (if (`self.HasMovementInput`)
    (return (`KismetMathLibrary.Conv_VectorToRotator` (`self.GetLastMovementInputVector`)))
    (else
      (return (`self.K2_GetActorRotation`)))))

(fn `InitializeFlow`
  (returns (Result :type Boolean))
  (while (== false (stale _result))
    (bind _result (`self.InitializeInventoryContent`)))
  (return true))

(fn `InitializeInventoryContent`
  (returns (Result :type Boolean))
  (bind _asbp_brunnhilde_player_game_mode (cast `/Game/Brunnhide/GameMode/BP_Brunnhilde_PlayerGameMode` (`GameplayStatics.GetGameMode`)))
  (bind _characterequipmentdataset (`/Game/Brunnhide/GameMode/BP_Brunnhilde_PlayerGameMode.CharacterEquipmentDataset` _asbp_brunnhilde_player_game_mode))
  (if (== (`KismetArrayLibrary.Array_Length` _characterequipmentdataset) 0)
    (return false)
    (else
      (for _array_element _characterequipmentdataset
        (bind _asitem (cast `Item` _array_element))
        (bind _returnvalue (`Item.DeepCopy` _asitem))
        (`InventoryComponent.AddItem` (`self.InventoryCmp`) _returnvalue))
      (return true))))

(fn `Start Rotation With Limit`
  (params (MaxPossibleRotation :type "Float (double-precision)") (MaxDegreeRotation :type "Float (double-precision)"))
  (return))

(fn `UserConstructionScript`)