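; Fighting NPC Blueprint for Brunnhilde that sets up the character's inventory, weapons and health display.
; InitializeFlow fills the inventory, equips every item, switches the state to Fighting, then creates the health widget.
; Health component change and death events are bound during setup, and UpdateHealthWidget writes current health into the widget.
; Tick and the construction script only call the parent, and ClearInventory is empty.
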(event `self.ReceiveTick`
  (params (DeltaSeconds :type "Float (single-precision)"))
  (`parent.ReceiveTick` DeltaSeconds))

(fn `ClearInventory`)

(fn `InitializeFlow`
  (returns (Result :type Boolean))
  (`self.InitializeInventoryContent`)
  (`self.SetupWeapon`)
  (`self.SetupHealthWidget`)
  (return true))

(fn `SetupHealthWidget`
  (bind _healthcmp (`self.HealthCmp`))
  (bind _returnvalue (`|CreateWidget` "/Game/Brunnhide/UserInterface/PlayerCharater/CharacterStats/WB_NPCHealthWidget.WB_NPCHealthWidget_C" null (`KismetMathLibrary.Conv_IntToDouble` (`HealthComponent.GetCurrentHealth` _healthcmp)) (`KismetMathLibrary.Conv_IntToDouble` (`HealthComponent.MaxHealth` _healthcmp))))
  (`WidgetComponent.SetWidget` (`self.HealthWidget`) _returnvalue)
  (add `HealthComponent.OnHealthChanged` _healthcmp (`|CreateDelegate` :!event `UpdateHealthWidget`))
  (add `HealthComponent.OnDied` _healthcmp (`|CreateDelegate` :!event `ClearInventory`))
  (return))

(fn `SetupWeapon`
  (for _array_element (`InventoryComponent.Items` (`self.InventoryCmp`))
    (`InventoryComponent.EquipItem` (`self.InventoryCmp`) _array_element))
  (set `self.CurrentState` "ECFSM_Fighting")
  (return))

(fn `UpdateHealthWidget`
  (params (Health :type Integer :default 0))
  (bind _aswb_npchealth_widget (cast `/Game/Brunnhide/UserInterface/PlayerCharater/CharacterStats/WB_NPCHealthWidget` (`WidgetComponent.GetUserWidgetObject` (`self.HealthWidget`))))
  (set `/Game/Brunnhide/UserInterface/PlayerCharater/CharacterStats/WB_NPCHealthWidget.CurrentHealth` (`KismetMathLibrary.Conv_IntToDouble` Health) _aswb_npchealth_widget))

(fn `UserConstructionScript`
  (`parent.UserConstructionScript`))