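; Brunnhilde mannequin NPC character that also carries player-style input for jumping, rolling, weapon pickup, enemy lock and heavy melee attack.
; On BeginPlay it spawns and equips a base weapon at the back socket and binds to health changes.
; Jump becomes a montage roll when moving, blocked during active montages.
; WASD sets dodge-direction flags, a helper updates the health widget, damage and rotation print debug text, and limited rotation is an empty stub.
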(event `self.ReceiveBeginPlay`
  (`self.EquipmentBaseWeapon`)
  (add `HealthComponent.OnHealthChanged` (`self.HealthCmp`) (`|CreateDelegate` :!event `UpdateHealthWidget`)))

(event `InputAction|PickUp`
  (params (Key :type "Key Structure"))
  ;[1 1 1] Pickup
  (:`Pressed`
    (`self.PickupWeapon`)))

(event `InputAction|LockEnemy`
  (params (Key :type "Key Structure"))
  ;[1 1 1] LockEnemy
  (:`Pressed`
    (`self.LockEnemy`)))

(event `InputAction|Jump`
  (params (Key :type "Key Structure"))
  ;[1 1 1] Jump & dodge
  (:`Pressed`
    (if (`self.HasMovementInput`)
      (`self.PlayRollAnimation`)
      (else
        (`self.Jump`))))
  (:`Released`
    (`self.StopJumping`)))

(event `Key|W`
  (params (Key :type "Key Structure"))
  ;[1 1 1] Dodge Direction
  (:`Pressed`
    (set `self.DodgeForward` true))
  (:`Released`
    (set `self.DodgeForward` false)))

(event `Key|D`
  (params (Key :type "Key Structure"))
  ;[1 1 1] Dodge Direction
  (:`Pressed`
    (set `self.DodgeRight` true))
  (:`Released`
    (set `self.DodgeRight` false)))

(event `Key|S`
  (params (Key :type "Key Structure"))
  ;[1 1 1] Dodge Direction
  (:`Pressed`
    (set `self.DodgeBackward` true))
  (:`Released`
    (set `self.DodgeBackward` false)))

(event `Key|A`
  (params (Key :type "Key Structure"))
  ;[1 1 1] Dodge Direction
  (:`Pressed`
    (set `self.DodgeLeft` true))
  (:`Released`
    (set `self.DodgeLeft` false)))

(event `self.ReceiveAnyDamage`
  (params (Damage :type "Float (single-precision)") (DamageType :type "DamageType Object Reference") (InstigatedBy :type "Controller Object Reference") (DamageCauser :type "Actor Object Reference"))
  (`KismetSystemLibrary.PrintString` (`KismetStringLibrary.Conv_IntToString` (`HealthComponent.GetCurrentHealth` (`self.HealthCmp`)))))

(event `InputAction|Roll`
  (params (Key :type "Key Structure"))
  ;[1 1 1] Roll
  (:`Pressed`
    (`self.PlayRollAnimation`)))

(event `InputAction|HeavyAttack`
  (params (Key :type "Key Structure"))
  ;[1 1 1] HeavyAttack
  (:`Pressed`
    (`self.MeleeAttack`)))

(fn `EquipmentBaseWeapon`
  (bind _returnvalue (`|SpawnActorFromClass` "/Game/Brunnhide/Weapon/BP_WeaponBase.BP_WeaponBase_C" (`SceneComponent.GetSocketTransform` (`self.Mesh`) "BACK_WEAPON" "RTS_World") "Undefined" "OverrideRootScale" self null))
  (`self.SetEquippedWeapon` _returnvalue))

(fn `GetDesiredRotation`
  (returns (Rotation :type "Rotator Structure"))
  (bind (_returnvalue_x _returnvalue_y _returnvalue_z) (`KismetMathLibrary.BreakVector` (`self.GetLastMovementInputVector`)))
  (`KismetSystemLibrary.PrintString` (`KismetTextLibrary.Conv_TextToString` (`|FormatText` "X:{ x}, Y:{y}, Z:{z}" (`KismetStringLibrary.Conv_DoubleToString` _returnvalue_x) (`KismetStringLibrary.Conv_DoubleToString` _returnvalue_y) (`KismetStringLibrary.Conv_DoubleToString` _returnvalue_z))))
  (if (`self.HasMovementInput`)
    (return (`KismetMathLibrary.Conv_VectorToRotator` (`self.GetLastMovementInputVector`)))
    (else
      (return (`self.K2_GetActorRotation`)))))

(fn `Start Rotation With Limit`
  (params (MaxPossibleRotation :type "Float (double-precision)") (MaxDegreeRotation :type "Float (double-precision)"))
  (return))

(fn `UpdateHealthWidget`
  (params (Health :type Integer))
  (bind _asui_npchealth_widget (cast `/Game/Brunnhide/UserInterface/CharacterStats/UI_NPCHealthWidget` (`WidgetComponent.GetUserWidgetObject` (`self.HealthWidget`))))
  (set `/Game/Brunnhide/UserInterface/CharacterStats/UI_NPCHealthWidget.CurrentHealth` (`KismetMathLibrary.Conv_IntToDouble` Health) _asui_npchealth_widget))

(fn `UserConstructionScript`)