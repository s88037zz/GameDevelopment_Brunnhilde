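; Player character Blueprint for Brunnhilde that can trigger a defender summoner through a test input action.
; On BeginPlay, InitializeFlow initializes inventory content, then spawns a visible BP_ColorChannel actor at the character's transform and stores it as the summoner.
; Pressing the TestActions input assigns the Brunnhilde defender base class to that summoner and calls its OnUse.
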(event `self.ReceiveBeginPlay`
  (`self.InitializeFlow`))

(event `InputAction|TestActions`
  (params (Key :type "Key Structure"))
  (bind _defendsummoner (`self.DefendSummoner`))
  (:`Pressed`
    (set `ColorChannel.DefenderBase` "/Game/Brunnhide/Character/NPC/FightingNPC/FightingNPC/Defender/BP_Brunnhilde_Defender_Base.BP_Brunnhilde_Defender_Base_C" _defendsummoner)
    (`ColorChannel.OnUse` _defendsummoner)))

(fn `InitializeFlow`
  (returns (Result :type Boolean))
  (`self.InitializeInventoryContent`)
  (`self.SetupDefenderSummoner`)
  (return true))

(fn `SetupDefenderSummoner`
  (returns (Result :type Boolean))
  (bind _returnvalue (`|SpawnActorFromClass` "/Game/Brunnhide/Character/Player/BP_ColorChannel.BP_ColorChannel_C" (`self.GetTransform`) "Undefined" "OverrideRootScale" null null))
  (`self.SetActorHiddenInGame` _returnvalue false)
  (set `self.DefendSummoner` _returnvalue)
  (return true))

(fn `UserConstructionScript`
  (`parent.UserConstructionScript`))