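; Enemy spawner actor that spawns waves of AI NPCs running NPC_BT, starting at its own transform on BeginPlay.
; A custom event spawns the configured number, then re-calls itself after a delay for endless rounds, without passing location or rotation on.
; Each spawned Brunnhilde mannequin NPC gets its FollowingPath from a loop over all BP_NPC_Pathway actors, so the last one found wins.
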(event `self.ReceiveBeginPlay`
  (`self.SpawnEnermy` (`self.EnermyClass`) (.location (`self.GetTransform`)) (.rotation (`self.GetTransform`)) (`self.Number Of Enermy`)))

(event `SpawnEnermy`
  (params (Class :type "Pawn Class Reference") (Location :type "Vector Structure") (Rotation :type "Rotator Structure") (`Number of Enermy` :type Integer))
  (for _ (range `Number of Enermy`)
    (bind _returnvalue (`AIBlueprintHelperLibrary.SpawnAIFromClass` Class "/Game/Brunnhide/Character/NPC/AIBehavior/NPC_BT.NPC_BT" Location Rotation false null))
    (bind _asbp_brunnhilde_mennequin_npc (cast `/Game/Brunnhide/Character/NPC/BP_Brunnhilde_Mennequin_NPC` _returnvalue))
    (`/Engine/EditorBlueprintResources/StandardMacros.IsValid` _asbp_brunnhilde_mennequin_npc
      (:`Is Valid`
        (bind _outactors (`GameplayStatics.GetAllActorsOfClass` "/Game/Brunnhide/Character/NPC/BP_NPC_Pathway.BP_NPC_Pathway_C"))
        (for _array_element _outactors
          (set `/Game/Brunnhide/Character/NPC/BP_Brunnhilde_Mennequin_NPC.FollowingPath` _array_element _asbp_brunnhilde_mennequin_npc)))))
  (`KismetSystemLibrary.Delay` (`self.DealyToSpawnNextRound`))
  (`self.SpawnEnermy` Class (0.0 0.0 0.0) (struct) (`self.Number Of Enermy`)))

(fn `UserConstructionScript`)