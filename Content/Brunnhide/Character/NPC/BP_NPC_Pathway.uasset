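; BP_NPC_Pathway is a spline path actor that moves a static mesh marker along its route, apparently as a guide for Brunnhilde NPCs.
; Each tick, unless paused, UpdateNewLocation advances the distance by speed times delta time and places the mesh at that spline point.
; Pause and Continue events toggle movement.
; A sphere overlap flags when an NPC is inside, though nothing here reads that flag.
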(event `Continue`
  (set `self.IsPause` false))

(event `Pause`
  (set `self.IsPause` true))

(event `self.ReceiveTick`
  (params (DeltaSeconds :type "Float (single-precision)"))
  (if (not (`self.IsPause`))
    (`self.UpdateNewLocation`)))

(event `self.Sphere.OnComponentBeginOverlap`
  (params (OverlappedComponent :type "PrimitiveComponent Object Reference") (OtherActor :type "Actor Object Reference") (OtherComp :type "PrimitiveComponent Object Reference") (OtherBodyIndex :type Integer) (bFromSweep :type Boolean) (SweepResult :type "HitResult Structure (by ref)"))
  (cast `/Game/Brunnhide/Character/NPC/BP_Brunnhilde_Mennequin_NPC` OtherActor)
  (set `self.OverrlappingNPC?` true))

(event `self.Sphere.OnComponentEndOverlap`
  (params (OverlappedComponent :type "PrimitiveComponent Object Reference") (OtherActor :type "Actor Object Reference") (OtherComp :type "PrimitiveComponent Object Reference") (OtherBodyIndex :type Integer))
  (cast `/Game/Brunnhide/Character/NPC/BP_Brunnhilde_Mennequin_NPC` OtherActor)
  (set `self.OverrlappingNPC?` false))

(fn `UserConstructionScript`)