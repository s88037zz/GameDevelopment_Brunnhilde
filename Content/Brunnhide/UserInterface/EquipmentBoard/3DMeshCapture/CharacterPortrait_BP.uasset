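; CharacterPortrait_BP is a stand-in actor that mirrors the player's Brunnhilde character, apparently for the equipment board's 3D portrait capture.
; On BeginPlay, UpdateCharacter casts the player pawn and copies its skeletal mesh onto the actor's own, resetting the pose.
; It then snaps its Helm component to the head socket and copies the player's helm mesh.
; No Tick logic runs, so the copy changes only when UpdateCharacter is called.
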(event `self.ReceiveBeginPlay`
  (`self.UpdateCharacter`))

(event `UpdateCharacter`
  (bind _asbp_brunnhilde_mennequin (cast `/Game/Brunnhide/Character/Mannequin/Blueprint/BP_Brunnhilde_Mennequin` (`GameplayStatics.GetPlayerPawn` 0)))
  (set `self.PlayerCharacter` _asbp_brunnhilde_mennequin)
  (`SkinnedMeshComponent.SetSkinnedAssetAndUpdate` (`self.SkeletalMesh`) (`SkinnedMeshComponent.SkeletalMesh` (`Character.Mesh` _asbp_brunnhilde_mennequin)) true)
  (`SceneComponent.K2_AttachToComponent` (`self.Helm`) (`self.SkeletalMesh`) "headSocket" "SnapToTarget" "SnapToTarget" "SnapToTarget" true)
  (`StaticMeshComponent.SetStaticMesh` (`self.Helm`) (`StaticMeshComponent.StaticMesh` (`/Game/Brunnhide/Character/Mannequin/Blueprint/BP_Brunnhilde_Mennequin.Helm` (`self.PlayerCharacter`)))))

(fn `UserConstructionScript`)