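; Enemy NPC character Blueprint for Brunnhilde that enters play armed and in a fighting state.
; After parent BeginPlay, SetupWeapon searches the inventory component for the first Weapon, equips it, sets the Fighting state and notifies the state machine of the drawn weapon.
; A separate UpdateHealthWidget function writes a given health value into the NPC health widget.
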(event `self.ReceiveBeginPlay`
  (`parent.ReceiveBeginPlay`)
  (`self.SetupWeapon`))

(fn `SetupWeapon`
  (for _array_element (`InventoryComponent.Items` (`self.InventoryCmp`))
    (bind _asweapon (cast `Weapon` _array_element))
    (`InventoryComponent.EquipItem` (`self.InventoryCmp`) _asweapon)
    (set `self.CurrentState` "ECFSM_Fighting")
    (bind _returnvalue (`self.GetStateMachine`))
    (`StateMachine.DrawnWeaponNotifcation` _returnvalue)
    (break)))

(fn `UpdateHealthWidget`
  (params (Health :type Integer))
  (bind _asui_npchealth_widget (cast `/Game/Brunnhide/UserInterface/CharacterStats/WB_NPCHealthWidget` (`WidgetComponent.GetUserWidgetObject` (`self.HealthWidget`))))
  (set `/Game/Brunnhide/UserInterface/CharacterStats/WB_NPCHealthWidget.CurrentHealth` (`KismetMathLibrary.Conv_IntToDouble` Health) _asui_npchealth_widget))

(fn `UserConstructionScript`
  (`parent.UserConstructionScript`))