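; BP_EnemySpawnor is an enemy spawner that produces endless rounds of AI enemies, starting on BeginPlay at its own transform.
; Its SpawnEnermy event spawns a set number of pawns of the configured class with a shared behavior tree.
; The event then calls itself after a configurable delay, passing only class and count, so later rounds do not receive the spawner's location or rotation.
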(event `self.ReceiveBeginPlay`
  (`self.SpawnEnermy` (`self.EnermyClass`) (.location (`self.GetTransform`)) (.rotation (`self.GetTransform`)) (`self.Number Of Enermy`)))

(event `SpawnEnermy`
  (params (Class :type "Pawn Class Reference") (Location :type "Vector Structure") (Rotation :type "Rotator Structure") (`Number of Enermy` :type Integer))
  (for _ (range `Number of Enermy`)
    (`AIBlueprintHelperLibrary.SpawnAIFromClass` Class (`self.EnermyBehaviorTree`) Location Rotation false null))
  (`KismetSystemLibrary.Delay` (`self.StartNextRoundDealyTime`))
  (`self.SpawnEnermy` Class (0.0 0.0 0.0) (struct) (`self.Number Of Enermy`)))

(fn `UserConstructionScript`)